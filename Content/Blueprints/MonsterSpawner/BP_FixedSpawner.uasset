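; Fixed monster spawner that places a BP_Enemy at a random SpawnPoints entry, only while no other BP_Enemy exists.
; Any overlap with EnterZone starts a looping timer with a randomized interval; the player overlapping EndZone, positioned by the construction script, clears it.
; If an enemy exists, the spawn event retries every half second.
; Location and rotation are rolled independently, and the ChanceDeAtaque roll yields State 0 either way.
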(event OnComponentBeginOverlap(EnterZone)
  (params (OverlappedComponent :type Primitive%20Component%20Object%20Reference) (OtherActor :type Actor%20Object%20Reference) (OtherComp :type Primitive%20Component%20Object%20Reference) (OtherBodyIndex :type Integer) (bFromSweep :type Boolean) (SweepResult :type Hit%20Result%20Structure%20%28by%20ref%29))
  (bind _returnvalue (Utilities|Time|SetTimerbyEvent (delegate Custom|Event_SpawnMonster) (Math|Random|RandomFloatinRange 1.0 (Variables|Settings|GetMaximoTiempoDeSpawn)) true))
  (Variables|Default|SetSpawnTimerHandle _returnvalue))

(event OnComponentBeginOverlap(EndZone)
  (params (OverlappedComponent :type Primitive%20Component%20Object%20Reference) (OtherActor :type Actor%20Object%20Reference) (OtherComp :type Primitive%20Component%20Object%20Reference) (OtherBodyIndex :type Integer) (bFromSweep :type Boolean) (SweepResult :type Hit%20Result%20Structure%20%28by%20ref%29))
  (if (== OtherActor (Game|GetPlayerCharacter 0))
    (Utilities|Time|ClearandInvalidateTimerbyHandle (Variables|Default|GetSpawnTimerHandle))))

(event Custom|Event_SpawnMonster
  (bind _outactors (Actor|GetAllActorsOfClass "/Game/Blueprints/MonsterSpawner/BP_Enemy.BP_Enemy_C" :!label _label))
  (if (== (Utilities|Array|Length _outactors) 0)
    (bind (_spawnpointloc _spawnpointrot) (CallFunction|GetSpawnpoint))
    (Game|SpawnActorfromClass "/Game/Blueprints/MonsterSpawner/BP_Enemy.BP_Enemy_C" (Math|Transform|MakeTransform _spawnpointloc _spawnpointrot "1,1,1") "Undefined" 0 (select (<= (Math|Random|RandomIntegerinRange 0 100) (Variables|Settings|GetChanceDeAtaque)) 0 0) 0)
    (else
      (Utilities|FlowControl|Delay 0.5)
      (goto _label))))

(event EventBeginPlay)

(fn ConstructionScript
  (Transformation|SetRelativeLocation (Variables|Default|GetEndZone) (Variables|Settings|GetEndZoneLocation) false false))

(fn GetSpawnpoint
  (bind _spawnpoints (Variables|Settings|GetSpawnPoints))
  (bind _spawnpoints_2 (Variables|Settings|GetSpawnPoints))
  (bind _returnvalue (Utilities|Array|Length _spawnpoints))
  (bind _returnvalue_2 (- _returnvalue 1))
  (bind _returnvalue_3 (Math|Random|RandomIntegerinRange 0 _returnvalue_2))
  (bind _output (Utilities|Array|Get(acopy) _spawnpoints_2 _returnvalue_3))
  (if (> (Utilities|Array|Length (Variables|Settings|GetSpawnPoints)) 0)
    (return (Transformation|GetActorLocation _output) (Transformation|GetActorRotation _output))))