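; BP_Enemy is a spawner enemy that picks Wandering or Attack behavior from its State at BeginPlay.
; Wandering disables box collision, tints it yellow and sends it far forward; Attack enables collision, tints it red, timeline-enlarges the mesh and targets the player's starting position.
; Movement is one AI MoveTo without pathfinding at zero Z, destroying the actor if already at goal.
; Overlap handling is empty, and navmesh path-following toward the player is unwired.
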(event OnComponentBeginOverlap(Box)
  (params (OverlappedComponent :type Primitive%20Component%20Object%20Reference) (OtherActor :type Actor%20Object%20Reference) (OtherComp :type Primitive%20Component%20Object%20Reference) (OtherBodyIndex :type Integer) (bFromSweep :type Boolean) (SweepResult :type Hit%20Result%20Structure%20%28by%20ref%29))
  (if (== OtherActor (Game|GetPlayerCharacter 0))
    _))

(event Custom|Event_MoveToward
  (params (Destination :type Vector))
  (bind _returnvalue (AI|Navigation|MovetoLocation (AI|GetAIController self) (Math|Vector|MakeVector (.x Destination) (.y Destination) 0.0) 1.0 true false false true 0))
  (switch Utilities|FlowControl|Switch|SwitchonEPathFollowingRequestResult _returnvalue
    (:Failed
      (Development|PrintString "Hello"))
    (:AlreadyAtGoal
      (Actor|DestroyActor))))

(event EventBeginPlay
  (switch Utilities|FlowControl|Switch|SwitchonE_MonsterState (Variables|Default|GetState)
    (:NewEnumerator0
      (CallFunction|WanderPointtoPoint))
    (:NewEnumerator1
      (CallFunction|AttackthePlayer)
      (bind _enlargecurve (Timeline|Enlarge PlayFromStart)
        (:Update
          (Transformation|SetWorldScale3D (Variables|Character|GetMesh) (Math|Vector|Lerp(Vector) "2.000000,2.000000,6.000000" "4.000000,4.000000,12.000000" _enlargecurve)))))))

(event EventTick
  (params (DeltaSeconds :type Float%20%28single-precision%29)))

(fn ConstructionScript
  (bind _returnvalue (Rendering|Material|CreateDynamicMaterialInstance (Variables|Character|GetMesh) 0 "/Game/Blueprints/MonsterSpawner/MT_EnemyMat.MT_EnemyMat" "None" :!class /Script/Engine.PrimitiveComponent))
  (Variables|Default|SetMaterial _returnvalue))

(fn GetNextPathPoint
  (bind _returnvalue (Class|NavigationSystemV1|FindPathtoActorSynchronously (Transformation|GetActorLocation) (Game|Player|GetPlayerPawn 0) 5e+01 0 0))
  (LocalVariables|SetLoc_Navpath _returnvalue)
  (if (> (Utilities|Array|Length (Variables|/Script/NavigationSystem.NavigationPath|GetPathPoints (LocalVariables|GetLoc_Navpath))) 1)
    (return (Utilities|Array|Get(acopy) (Variables|/Script/NavigationSystem.NavigationPath|GetPathPoints (LocalVariables|GetLoc_Navpath)) 1))
    (else
      (return (Transformation|GetActorLocation)))))

(fn WanderPointtoPoint
  (Collision|SetCollisionEnabled (Variables|Default|GetBox) "NoCollision")
  (CallFunction|SetColor "(R=0.458333,G=0.386896,B=0.000000,A=1.000000)")
  (CallFunction|EventMoveToward (+ (Transformation|GetActorLocation) (* (Transformation|GetActorForwardVector) 1.6e+04))))

(fn AttackthePlayer
  (Collision|SetCollisionEnabled (Variables|Default|GetBox) "QueryAndPhysics")
  (CallFunction|SetColor "(R=0.458333,G=0.000000,B=0.019881,A=1.000000)")
  (Variables|/Script/Engine.CharacterMovementComponent|SetMaxFlySpeed (Variables|Character|GetCharacterMovement) 4e+02)
  (CallFunction|EventMoveToward (Transformation|GetActorLocation (Game|GetPlayerCharacter 0))))

(fn SetColor
  (params (Value :type Linear%20Color%20Structure :default "(R=0.458333,G=0.386896,B=0.000000,A=1.000000)"))
  (Rendering|Material|SetVectorParameterValue (Variables|Default|GetMaterial) "Color" Value :!class /Script/Engine.MaterialInstanceDynamic))