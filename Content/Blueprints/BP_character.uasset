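; BP_character is a player-controlled Character handling basic movement, camera look, running, jumping and quitting the game.
; Axis inputs drive movement along actor forward and right vectors, with direct mouse look and frame-time-scaled stick look rates.
; Holding Run raises walk speed to RunSpeed, and release restores a hardcoded default.
; Jump copies JumpHeight into JumpMaxHoldTime before jumping, with no release handler, and Escape quits immediately.
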(event EventBeginPlay)

(event Collision|EventActorBeginOverlap
  (params (OtherActor :type Actor%20Object%20Reference)))

(event EventTick
  (params (DeltaSeconds :type Float%20%28single-precision%29)))

(event Input|ActionEvents|InputActionJump
  (params (Key :type Key%20Structure :default "None"))
  ;[1 1 1] Run And Jump
  (:Pressed
    (Variables|Default|SetJumpMaxHoldTime (Variables|Default|GetJumpHeight))
    (Character|Jump)))

(event Input|ActionEvents|InputActionEscape
  (params (Key :type Key%20Structure :default "None"))
  (:Pressed
    (Game|QuitGame 0 "Quit" false)))

(event Input|ActionEvents|InputActionRun
  (params (Key :type Key%20Structure :default "None"))
  (bind _charactermovement (Variables|Character|GetCharacterMovement))
  ;[1 1 1] Run And Jump
  (:Pressed
    (Variables|/Script/Engine.CharacterMovementComponent|SetMaxWalkSpeed _charactermovement (Variables|Default|GetRunSpeed)))
  (:Released
    (Variables|/Script/Engine.CharacterMovementComponent|SetMaxWalkSpeed _charactermovement 4e+02)))

(event Input|AxisEvents|InputAxisMoveForward
  (params (AxisValue :type Float%20%28single-precision%29))
  ;[1 1 1] Movimiento
  (Pawn|Input|AddMovementInput (Transformation|GetActorForwardVector) AxisValue false))

(event Input|AxisEvents|InputAxisMoveRight
  (params (AxisValue :type Float%20%28single-precision%29))
  ;[1 1 1] Movimiento
  (Pawn|Input|AddMovementInput (Transformation|GetActorRightVector) AxisValue false))

(event Input|AxisEvents|InputAxisTurn
  (params (AxisValue :type Float%20%28single-precision%29))
  ;[1 1 1] Mouse Movement
  (Pawn|Input|AddControllerYawInput AxisValue))

(event Input|AxisEvents|InputAxisLookUp
  (params (AxisValue :type Float%20%28single-precision%29))
  ;[1 1 1] Mouse Movement
  (Pawn|Input|AddControllerPitchInput AxisValue))

(event Input|AxisEvents|InputAxisLookUpRate
  (params (AxisValue :type Float%20%28single-precision%29))
  ;[1 1 1] Stick Controllers
  (Pawn|Input|AddControllerPitchInput (* AxisValue (Variables|Default|GetBase%20Look%20UP%20Rate) (Utilities|Time|GetWorldDeltaSeconds))))

(event Input|AxisEvents|InputAxisTurnRate
  (params (AxisValue :type Float%20%28single-precision%29))
  ;[1 1 1] Stick Controllers
  (Pawn|Input|AddControllerYawInput (* AxisValue (Variables|Default|GetBase%20Turn%20Rate) (Utilities|Time|GetWorldDeltaSeconds))))

(fn ConstructionScript)